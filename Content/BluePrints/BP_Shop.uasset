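; BP_Shop is a shop display where the player cycles items with R/F and presses E to shop using their character's TotalCoins.
; ShopObject and the item-change functions are called here but defined elsewhere, with collect and change events driving the visuals.
; One Timeline animates item scale; on a change, its rebound finished callback swaps mesh and target scale, then reverses the animation.
; BeginPlay runs that swap to show the initial item.
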(event `Key|E`
  (params (Key :type "Key Structure"))
  (:`Pressed`
    (bind _asbp_third_person_character (cast `/Game/ThirdPerson/Blueprints/BP_ThirdPersonCharacter` (`GameplayStatics.GetPlayerCharacter` 0)))
    (`self.ShopObject` (`ScriptingExercisesCharacter.TotalCoins` _asbp_third_person_character))))

(event `self.OnObjectCollected`
  (bind (_direction _newtrack_0) (`Timeline|Timeline` :!via `PlayFromStart`)
    (:`Update`
      (`SceneComponent.SetRelativeScale3D` (`self.Item`) (`KismetMathLibrary.Conv_DoubleToVector` (`KismetMathLibrary.Lerp` 0.0 (`self.CurrentItemScale`) _newtrack_0))))))

(event `Key|F`
  (params (Key :type "Key Structure"))
  (:`Pressed`
    (`self.ChangeItemDown`)))

(event `Key|R`
  (params (Key :type "Key Structure"))
  (:`Pressed`
    (`self.ChangeItemUp`)))

(event `self.OnChangeItem`
  (bind _timeline (`self.Timeline`))
  (`TimelineComponent.PlayFromStart` _timeline)
  (`TimelineComponent.SetTimelineFinishedFunc` _timeline (delegate `OnTimelineChangeItemFinished`)))

(event `OnTimelineChangeItemFinished`
  (bind _timeline (`self.Timeline`))
  (bind (_output_name _output_description _output_cost _output_itemscale _output_itemmesh) (break `CCItemInfo` (`|GetArrayItem` (`self.Items`) (`self.ItemIndex`))))
  (set `self.CurrentItemScale` _output_itemscale)
  (`StaticMeshComponent.SetStaticMesh` (`self.Item`) _output_itemmesh)
  (`TimelineComponent.ReverseFromEnd` _timeline)
  (`TimelineComponent.SetTimelineFinishedFunc` :`self` _timeline))

(event `self.ReceiveBeginPlay`
  (`self.OnTimelineChangeItemFinished`))

(fn `UserConstructionScript`)